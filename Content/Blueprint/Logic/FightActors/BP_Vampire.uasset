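; Vampire fight actor that plays the visuals and audio for its combat actions and poison status.
; PlayNextActionAnim switches on action type: each attack sets a material frame, activates its own VFX and runs a timeline that slides the mesh along Y, fires a timed sound and resets the frame.
; Status events toggle poison VFX and a Poisoned material parameter when the first copy is applied or the last removed.
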(event `self.ReceivePlayNextActionAnim`
  (params (InActionType :type "EActionType Enum (by ref)" :default "None"))
  (switch `EActionType` InActionType
    (:`Bite`
      ; MeleeAttack
      ;; VampireBiteAttack
      (`MeshComponent.SetScalarParameterValueOnMaterials` (`self.ActorMesh`) "Frame" 3.0)
      (`MeshComponent.SetScalarParameterValueOnMaterials` (`self.ActorMesh`) "CharacterSwitch" 1.0)
      (`ActorComponent.Activate` (`self.VFX_Attack_Bite`) true)
      (bind (_direction _vampireattackmovement) (`Timeline|Timeline_0` :!via `PlayFromStart`)
        (:`Update`
          (`SceneComponent.K2_SetRelativeLocation` (`self.ActorMesh`) (`KismetMathLibrary.MakeVector` 0.0 (* _vampireattackmovement 300.0)) false false))
        (:`Finished`
          (`MeshComponent.SetScalarParameterValueOnMaterials` (`self.ActorMesh`) "Frame" 1.0))
        (:`BiteSound`
          (`GameplayStatics.PlaySoundAtLocation` "/Game/Assets/Audio/Sounds/Attacks/MSS_Attack_Bite.MSS_Attack_Bite" (`self.K2_GetActorLocation`) (struct) 1.0 1.0 0.0 null null null null))))
    (:`PoisonStrike`
      ; Range Attack
      ;; VampirePoisonAttack
      (`MeshComponent.SetScalarParameterValueOnMaterials` (`self.ActorMesh`) "Frame" 4.0)
      (`MeshComponent.SetScalarParameterValueOnMaterials` (`self.ActorMesh`) "CharacterSwitch" 1.0)
      (`ActorComponent.Activate` (`self.VFX_Attack_Poison`) true)
      (bind (_direction_2 _vampireattackmovement_2 _charahitmovement _hitcolor _charamovementblocking _vampirehitmovement _vampirerangemovement) (`Timeline|Timeline_1` :!via `PlayFromStart`)
        (:`Update`
          (`SceneComponent.K2_SetRelativeLocation` (`self.ActorMesh`) (`KismetMathLibrary.MakeVector` 0.0 (* _vampirerangemovement 300.0)) false false))
        (:`Finished`
          (`MeshComponent.SetScalarParameterValueOnMaterials` (`self.ActorMesh`) "Frame" 1.0))
        (:`DartsSound`
          (`GameplayStatics.PlaySoundAtLocation` "/Game/Assets/Audio/Sounds/Attacks/MSS_Attack_Poison_Darts.MSS_Attack_Poison_Darts" (`self.K2_GetActorLocation`) (struct) 1.0 1.0 0.0 null null null null))))
    (:`SeethingPoison`
      ;; VampireBoilingAttack
      (`MeshComponent.SetScalarParameterValueOnMaterials` (`self.ActorMesh`) "Frame" 4.0)
      (`MeshComponent.SetScalarParameterValueOnMaterials` (`self.ActorMesh`) "CharacterSwitch" 1.0)
      (`ActorComponent.Activate` (`self.VFX_Attack_Boiling`) true)
      (bind (_direction_3 _vampireattackmovement_3 _charahitmovement_2 _hitcolor_2 _charamovementblocking_2 _vampirehitmovement_2 _vampirerangemovement_2) (`Timeline|Timeline_2` :!via `PlayFromStart`)
        (:`Update`
          (`SceneComponent.K2_SetRelativeLocation` (`self.ActorMesh`) (`KismetMathLibrary.MakeVector` 0.0 (* _vampirerangemovement_2 300.0)) false false))
        (:`Finished`
          (`MeshComponent.SetScalarParameterValueOnMaterials` (`self.ActorMesh`) "Frame" 1.0))
        (:`BoilingSound`
          (`GameplayStatics.PlaySoundAtLocation` "/Game/Assets/Audio/Sounds/Attacks/MSS_Attack_Boiling.MSS_Attack_Boiling" (`self.K2_GetActorLocation`) (struct) 1.0 1.0 0.0 null null null null))))
    (:`Claws`
      ;; VampireClawsAttack
      (`MeshComponent.SetScalarParameterValueOnMaterials` (`self.ActorMesh`) "Frame" 3.0)
      (`MeshComponent.SetScalarParameterValueOnMaterials` (`self.ActorMesh`) "CharacterSwitch" 1.0)
      (`ActorComponent.Activate` (`self.VFX_Attack_Claws`) true)
      (bind (_direction_4 _vampireattackmovement_4) (`Timeline|Timeline` :!via `PlayFromStart`)
        (:`Update`
          (`SceneComponent.K2_SetRelativeLocation` (`self.ActorMesh`) (`KismetMathLibrary.MakeVector` 0.0 (* _vampireattackmovement_4 300.0)) false false))
        (:`Finished`
          (`MeshComponent.SetScalarParameterValueOnMaterials` (`self.ActorMesh`) "Frame" 1.0))
        (:`ClawsSound`
          (`GameplayStatics.PlaySoundAtLocation` "/Game/Assets/Audio/Sounds/Attacks/MSS_Attack_Claws.MSS_Attack_Claws" (`self.K2_GetActorLocation`) (struct) 1.0 1.0 0.0 null null null null))))
    (:`PsychicHorrorEvocation`
      ;; VampireMadnessAttack
      (`MeshComponent.SetScalarParameterValueOnMaterials` (`self.ActorMesh`) "Frame" 4.0)
      (`MeshComponent.SetScalarParameterValueOnMaterials` (`self.ActorMesh`) "CharacterSwitch" 1.0)
      (`ActorComponent.Activate` (`self.VFX_Attack_Madness`) true)
      (bind (_direction_5 _vampireattackmovement_5 _charahitmovement_3 _hitcolor_3 _charamovementblocking_3 _vampirehitmovement_3 _vampirerangemovement_3) (`Timeline|Timeline_3` :!via `PlayFromStart`)
        (:`Update`
          (`SceneComponent.K2_SetRelativeLocation` (`self.ActorMesh`) (`KismetMathLibrary.MakeVector` 0.0 (* _vampirerangemovement_3 300.0)) false false))
        (:`Finished`
          (`MeshComponent.SetScalarParameterValueOnMaterials` (`self.ActorMesh`) "Frame" 1.0))
        (:`WordsOfMadnessSound`
          (`GameplayStatics.PlaySoundAtLocation` "/Game/Assets/Audio/SoundBank/Attack_Song_of_madness.Attack_Song_of_madness" (`self.K2_GetActorLocation`) (struct) 1.0 1.0 0.0 null null null null))))
    (:`MentalClaws`
      ;; VampireConfusionAttack
      (`MeshComponent.SetScalarParameterValueOnMaterials` (`self.ActorMesh`) "Frame" 4.0)
      (`MeshComponent.SetScalarParameterValueOnMaterials` (`self.ActorMesh`) "CharacterSwitch" 1.0)
      (`ActorComponent.Activate` (`self.VFX_Attack_Confusion`) true)
      (bind (_direction_6 _vampireattackmovement_6 _charahitmovement_4 _hitcolor_4 _charamovementblocking_4 _vampirehitmovement_4 _vampirerangemovement_4) (`Timeline|Timeline_4` :!via `PlayFromStart`)
        (:`Update`
          (`SceneComponent.K2_SetRelativeLocation` (`self.ActorMesh`) (`KismetMathLibrary.MakeVector` 0.0 (* _vampirerangemovement_4 300.0)) false false))
        (:`Finished`
          (`MeshComponent.SetScalarParameterValueOnMaterials` (`self.ActorMesh`) "Frame" 1.0))
        (:`ConfusionSound`
          (`GameplayStatics.PlaySoundAtLocation` "/Game/Assets/Audio/Sounds/Attacks/MSS_Attack_Confusion.MSS_Attack_Confusion" (`self.K2_GetActorLocation`) (struct) 1.0 1.0 0.0 null null null null))))))

(event `self.ReceiveOnFirstStatusCopyApplied`
  (params (StatusEnum :type "EStatusEnum Enum (by ref)" :default "ST_None"))
  (switch `EStatusEnum` StatusEnum
    (:`ST_Poison`
      ; VampireStatusPoison
      (`MeshComponent.SetScalarParameterValueOnMaterials` (`self.ActorMesh`) "CharacterSwitch" 1.0)
      (`ActorComponent.Activate` (`self.VFX_Status_Poison`) true)
      (`MeshComponent.SetScalarParameterValueOnMaterials` (`self.ActorMesh`) "Poisoned" 1.0))))

(event `self.ReceiveOnLastStatusCopyRemoved`
  (params (StatusEnum :type "EStatusEnum Enum (by ref)" :default "ST_None"))
  (switch `EStatusEnum` StatusEnum
    (:`ST_Poison`
      ; VampireStatusPoisonRemoval
      (`MeshComponent.SetScalarParameterValueOnMaterials` (`self.ActorMesh`) "CharacterSwitch" 1.0)
      (`ActorComponent.Deactivate` (`self.VFX_Status_Poison`))
      (`MeshComponent.SetScalarParameterValueOnMaterials` (`self.ActorMesh`) "Poisoned" 0.0))))

(fn `UserConstructionScript`)