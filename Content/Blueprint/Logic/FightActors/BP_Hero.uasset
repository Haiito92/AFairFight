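; Hero fight actor Blueprint that plays the hero's visual reactions to combat actions and status effects.
; Pass and Block actions switch the sprite frame through material scalars and run timelines that shift the mesh along Y, then restore the frame.
; Pass also tints the mesh as a hit reaction, while Block activates a shield VFX.
; First-applied and last-removed Poison or Confused statuses toggle matching VFX and material parameters.
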(event `self.ReceivePlayNextActionAnim`
  (params (InActionType :type "EActionType Enum (by ref)" :default "None"))
  (switch `EActionType` InActionType
    (:`Pass`
      ; HeroAnim
      ;; CharaHit
      (`MeshComponent.SetScalarParameterValueOnMaterials` (`self.ActorMesh`) "Frame" 2.0)
      (`MeshComponent.SetScalarParameterValueOnMaterials` (`self.ActorMesh`) "CharacterSwitch" 0.0)
      (bind (_direction _vampireattackmovement _charahitmovement _hitcolor) (`Timeline|Timeline_0` :!via `PlayFromStart`)
        (:`Update`
          (`SceneComponent.K2_SetRelativeLocation` (`self.ActorMesh`) (`KismetMathLibrary.MakeVector` 0.0 (* _charahitmovement 300.0)) false false)
          (`MeshComponent.SetVectorParameterValueOnMaterials` (`self.ActorMesh`) "ColorMultiply" (`KismetMathLibrary.Conv_LinearColorToVector` _hitcolor)))
        (:`Finished`
          (`MeshComponent.SetScalarParameterValueOnMaterials` (`self.ActorMesh`) "Frame" 1.0))))
    (:`Block`
      ;; Blocking
      (`MeshComponent.SetScalarParameterValueOnMaterials` (`self.ActorMesh`) "Frame" 3.0)
      (`MeshComponent.SetScalarParameterValueOnMaterials` (`self.ActorMesh`) "CharacterSwitch" 0.0)
      (`ActorComponent.Activate` (`self.VFX_Shield`) true)
      (bind (_direction_2 _charahitmovement_2 _hitcolor_2 _charamovementblocking) (`Timeline|Timeline` :!via `PlayFromStart`)
        (:`Update`
          (`SceneComponent.K2_SetRelativeLocation` (`self.ActorMesh`) (`KismetMathLibrary.MakeVector` 0.0 (* _charamovementblocking 300.0)) false false))
        (:`Finished`
          (`MeshComponent.SetScalarParameterValueOnMaterials` (`self.ActorMesh`) "Frame" 1.0))))))

(event `self.ReceiveOnFirstStatusCopyApplied`
  (params (StatusEnum :type "EStatusEnum Enum (by ref)" :default "ST_None"))
  (switch `EStatusEnum` StatusEnum
    (:`ST_Poison`
      ; HeroStatusPoison
      (`MeshComponent.SetScalarParameterValueOnMaterials` (`self.ActorMesh`) "CharacterSwitch" 0.0)
      (`ActorComponent.Activate` (`self.VFX_Status_Poison`) true)
      (`MeshComponent.SetScalarParameterValueOnMaterials` (`self.ActorMesh`) "Poisoned" 1.0))
    (:`ST_Confused`
      ; HeroConfusedPoison
      (`MeshComponent.SetScalarParameterValueOnMaterials` (`self.ActorMesh`) "CharacterSwitch" 0.0)
      (`ActorComponent.Activate` (`self.VFX_Status_Confusion`) true)
      (`MeshComponent.SetScalarParameterValueOnMaterials` (`self.ActorMesh`) "Confused" 1.0))))

(event `self.ReceiveOnLastStatusCopyRemoved`
  (params (StatusEnum :type "EStatusEnum Enum (by ref)" :default "ST_None"))
  (switch `EStatusEnum` StatusEnum
    (:`ST_Poison`
      ; HeroStatusPoisonDeactivate
      (`MeshComponent.SetScalarParameterValueOnMaterials` (`self.ActorMesh`) "CharacterSwitch" 0.0)
      (`ActorComponent.Deactivate` (`self.VFX_Status_Poison`))
      (`MeshComponent.SetScalarParameterValueOnMaterials` (`self.ActorMesh`) "Poisoned" 0.0))
    (:`ST_Confused`
      ; HeroConfusedPoisonDeactivate
      (`MeshComponent.SetScalarParameterValueOnMaterials` (`self.ActorMesh`) "CharacterSwitch" 0.0)
      (`ActorComponent.Deactivate` (`self.VFX_Status_Confusion`))
      (`MeshComponent.SetScalarParameterValueOnMaterials` (`self.ActorMesh`) "Confused" 0.0))))

(fn `UserConstructionScript`)